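; MultiDoor is a double door that swings its two leaves open in opposite directions.
; BeginPlay caches each leaf's closed world rotation and an open rotation offset a quarter turn in yaw.
; The OpenDoor event plays the opening sound, deactivates the particle system, and runs a timeline that lerps both leaves between those rotations along the shortest path.
; The file contains no closing logic.
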(event EventBeginPlay
  (bind _left (Variables|Default|Getleft))
  (bind _right (Variables|Default|Getright))
  (bind _returnvalue (Transformation|GetWorldRotation _left))
  (bind _returnvalue_2 (Transformation|GetWorldRotation _right))
  (bind (_roll _pitch _yaw) (Math|Rotator|BreakRotator _returnvalue))
  (bind (_roll_2 _pitch_2 _yaw_2) (Math|Rotator|BreakRotator _returnvalue_2))
  (Variables|Default|Setleft_initPos (Transformation|GetWorldRotation _left))
  (Variables|Default|Setleft_finalPos (Math|Rotator|MakeRotator _roll _pitch (+ _yaw -9e+01)))
  (Variables|Default|Setright_initPos (Transformation|GetWorldRotation _right))
  (Variables|Default|Setright_finalPos (Math|Rotator|MakeRotator _roll_2 _pitch_2 (+ _yaw_2 9e+01))))

(event EventOpenDoor
  (Audio|Components|Audio|Play (Variables|Default|GetDoor-opening) 0.0)
  (Components|Activation|Deactivate (Variables|Default|GetParticleSystem))
  (bind _open_multidoor_track (Timeline|Timeline_0 Play)
    (:Update
      (Transformation|SetWorldRotation (Variables|Default|Getleft) (Math|Rotator|Lerp(Rotator) (Variables|Default|Getleft_initPos) (Variables|Default|Getleft_finalPos) _open_multidoor_track true) false false)
      (Transformation|SetWorldRotation (Variables|Default|Getright) (Math|Rotator|Lerp(Rotator) (Variables|Default|Getright_initPos) (Variables|Default|Getright_finalPos) _open_multidoor_track true) false false))))

(fn ConstructionScript
  (|CallParentFunction))