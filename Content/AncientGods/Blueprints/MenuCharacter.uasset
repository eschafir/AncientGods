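; MenuCharacter is the main menu's character Blueprint, which shows the menu and fades it along with the scene.
; On BeginPlay it adds MainMenuWidget to the viewport, shows the cursor and switches input to UI only.
; The FadeOut timeline then drives both FirstPersonCamera's post-process Gain and the widget's opacity from one FadeTime track.
; The FadeIn event plays that timeline in reverse.
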(event Custom|FadeIn
  (bind _fadetime (Timeline|FadeOut Reverse)
    (:Update
      (Utilities|Struct|SetmembersinPostProcessSettings (Variables|/Script/Engine.CameraComponent|GetPostProcessSettings (Variables|MyCharacter|GetFirstPersonCamera)) (Math|Vector4|MakeVector4 _fadetime _fadetime _fadetime _fadetime))
      (Appearance|SetColorandOpacity (Variables|Default|GetMenuWidget) (Math|Color|MakeColor 1.0 1.0 1.0 _fadetime) :!class /Script/UMG.UserWidget))))

(event EventBeginPlay
  (bind _returnvalue (Game|GetPlayerController 0))
  (bind _returnvalue_2 (UserInterface|CreateWidget "/Game/AncientGods/UI/MainMenuWidget.MainMenuWidget_C"))
  (bind _output_get (Variables|Default|SetMenuWidget _returnvalue_2))
  (UserInterface|Viewport|AddtoViewport _output_get 0)
  (Variables|/Script/Engine.PlayerController|SetbShowMouseCursor _returnvalue true)
  (Input|SetInputModeUIOnly _returnvalue (Variables|Default|GetMenuWidget) "DoNotLock")
  (bind _fadetime (Timeline|FadeOut PlayFromStart)
    (:Update
      (Utilities|Struct|SetmembersinPostProcessSettings (Variables|/Script/Engine.CameraComponent|GetPostProcessSettings (Variables|MyCharacter|GetFirstPersonCamera)) (Math|Vector4|MakeVector4 _fadetime _fadetime _fadetime _fadetime))
      (Appearance|SetColorandOpacity (Variables|Default|GetMenuWidget) (Math|Color|MakeColor 1.0 1.0 1.0 _fadetime) :!class /Script/UMG.UserWidget))))

(fn ConstructionScript)