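; Collectible star pickup that grants extra time and registers itself in the player character's level-wide star total on BeginPlay.
; The first overlap of its box, not filtered by actor, hides it, plays a sound, fades its proximity loop, spawns an explosion and calls CountStars on the character.
; It then adds TimeAdd to the HUD's extra time and tints the timer border through a color timeline.
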(event OnComponentBeginOverlap(Box)
  (params (OverlappedComponent :type Primitive%20Component%20Object%20Reference) (OtherActor :type Actor%20Object%20Reference) (OtherComp :type Primitive%20Component%20Object%20Reference) (OtherBodyIndex :type Integer) (bFromSweep :type Boolean) (SweepResult :type Hit%20Result%20Structure%20%28by%20ref%29))
  (Utilities|FlowControl|DoOnce false
    (:Completed
      (Rendering|SetActorHiddenInGame true)
      (Audio|Components|Audio|Play (Variables|Default|Getitem_pickup) 0.0)
      (Audio|Components|Audio|FadeOut (Variables|Default|GetProximity-Loop) 2.0 0.0 :!class /Script/Engine.AudioComponent)
      (Effects|SpawnEmitteratLocation "/Game/StarterContent/Particles/P_Explosion.P_Explosion" (Transformation|GetActorLocation) "0, 0, 0" "1.200000,1.200000,1.200000")
      (Default|CountStars (.AsFirst%20Person%20Character (Utilities|Casting|CastToFirstPersonCharacter (Game|GetPlayerCharacter 0))))
      (CallFunction|UpdateHud))))

(event Custom|UpdateHud
  ;[1 1 1] Updates de Player HUD when he takes a Pickup. The timer changes its color and adds extra time, based on the pickup.
  (bind _asfirst_person_character (Utilities|Casting|CastToFirstPersonCharacter (Game|GetPlayerCharacter 0)))
  (Variables|/Game/AncientGods/UI/PlayerUI.PlayerUI_C|SetExtraTime (Variables|/Game/FirstPersonBP/Blueprints/FirstPersonCharacter.FirstPersonCharacter_C|GetCharacterUI _asfirst_person_character) (+ (Variables|/Game/AncientGods/UI/PlayerUI.PlayerUI_C|GetExtraTime (Variables|/Game/FirstPersonBP/Blueprints/FirstPersonCharacter.FirstPersonCharacter_C|GetCharacterUI _asfirst_person_character)) (Variables|Default|GetTimeAdd)))
  (bind _alphacolor (Timeline|ColorChanger PlayFromStart)
    (:Update
      (Class|Border|SetBrushColor (Variables|/Game/AncientGods/UI/PlayerUI.PlayerUI_C|GetTimeBorder (Variables|/Game/FirstPersonBP/Blueprints/FirstPersonCharacter.FirstPersonCharacter_C|GetCharacterUI _asfirst_person_character)) (Math|Color|Lerp(LinearColor) "(R=0.000000,G=0.000000,B=0.000000,A=0.500000)" "(R=0.857143,G=0.244937,B=0.000000,A=1.000000)" _alphacolor)))))

(event EventBeginPlay
  (bind _returnvalue (Game|GetPlayerCharacter 0))
  (bind _asfirst_person_character (Utilities|Casting|CastToFirstPersonCharacter _returnvalue))
  ;[1 1 1] When a new instance of pickup class is created, it adds +1 to the global counter.
  (bind _result (Math|Integer|IncrementInt (Variables|/Game/FirstPersonBP/Blueprints/FirstPersonCharacter.FirstPersonCharacter_C|GetTotalStarsInLevel _asfirst_person_character))
    (:%20%20
      (Variables|/Game/FirstPersonBP/Blueprints/FirstPersonCharacter.FirstPersonCharacter_C|SetTotalStarsInLevel _asfirst_person_character _result))))

(fn ConstructionScript)