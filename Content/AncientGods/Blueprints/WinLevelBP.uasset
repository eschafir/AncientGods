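; WinLevelBP is the level's winning-point actor, ending the level when its box is overlapped and loading NextLevel.
; The overlap sets GameIsOver on the FirstPersonCharacter and hides its timer and pickup HUD widgets.
; A DoOnce then plays victory audio, fades out the loop sound and sets the game instance's fade color to white.
; The FadeIn timeline runs in reverse to fade the screen to white before opening the next level.
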(event OnComponentBeginOverlap(Box)
  (params (OverlappedComponent :type Primitive%20Component%20Object%20Reference) (OtherActor :type Actor%20Object%20Reference) (OtherComp :type Primitive%20Component%20Object%20Reference) (OtherBodyIndex :type Integer) (bFromSweep :type Boolean) (SweepResult :type Hit%20Result%20Structure%20%28by%20ref%29))
  (bind _returnvalue (Game|GetPlayerCharacter 0))
  (bind _asfirst_person_character (Utilities|Casting|CastToFirstPersonCharacter _returnvalue))
  ;[1 1 1] This occurs when the player touches the Winning point.
  (Variables|/Game/FirstPersonBP/Blueprints/FirstPersonCharacter.FirstPersonCharacter_C|SetGameIsOver? _asfirst_person_character true)
  (Widget|SetVisibility (Variables|/Game/AncientGods/UI/PlayerUI.PlayerUI_C|GetTimeBorder (Variables|/Game/FirstPersonBP/Blueprints/FirstPersonCharacter.FirstPersonCharacter_C|GetCharacterUI _asfirst_person_character)) "Hidden")
  (Utilities|FlowControl|DoOnce false
    (:Completed
      (Variables|/Game/AncientGods/Blueprints/TheStarterGameInstance.TheStarterGameInstance_C|SetFade%20Color (.AsThe%20Starter%20Game%20Instance (Utilities|Casting|CastToTheStarterGameInstance (Game|GetGameInstance))) "(R=1.000000,G=1.000000,B=1.000000,A=1.000000)")
      (Audio|Components|Audio|Play (Variables|Default|Getrelampago-victory) 0.0)
      (Audio|Components|Audio|FadeOut (Variables|Default|GetRelampago-loop) 1.5 0.0 :!class /Script/Engine.AudioComponent)
      (bind _fader (Timeline|FadeIn ReverseFromEnd)
        (:Update
          (bind _asfirst_person_character_2 (Utilities|Casting|CastToFirstPersonCharacter (Game|GetPlayerCharacter 0)))
          (Class|Border|SetBrushColor (Variables|/Game/AncientGods/UI/PlayerUI.PlayerUI_C|GetFader (Variables|/Game/FirstPersonBP/Blueprints/FirstPersonCharacter.FirstPersonCharacter_C|GetCharacterUI _asfirst_person_character_2)) (Math|Color|Lerp(LinearColor) (Variables|/Game/AncientGods/Blueprints/TheStarterGameInstance.TheStarterGameInstance_C|GetFade%20Color (.AsThe%20Starter%20Game%20Instance (Utilities|Casting|CastToTheStarterGameInstance (Game|GetGameInstance)))) "(R=0.000000,G=0.000000,B=0.000000,A=0.000000)" _fader)))
        (:Finished
          (Game|OpenLevel(byName) (Variables|Default|GetNext%20Level)))))))

(event EventBeginPlay)

(event Collision|EventActorBeginOverlap
  (params (OtherActor :type Actor%20Object%20Reference)))

(event EventTick
  (params (DeltaSeconds :type Float%20%28single-precision%29)))

(fn ConstructionScript)