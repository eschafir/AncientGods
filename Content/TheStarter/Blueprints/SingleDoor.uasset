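; SingleDoor is a door actor that rises vertically when its OpenDoor event is called.
; BeginPlay caches the starting location and a target at a fixed height above it.
; OpenDoor plays the Dooropening component, deactivates the particle system, and restarts a timeline that lerps the whole actor between the two points without sweeping.
; The file has no closing logic.
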(event EventBeginPlay
  (bind _returnvalue (Transformation|GetActorLocation))
  (Variables|Default|SetInitPos _returnvalue)
  (Variables|Default|SetFinalPos (+ _returnvalue "0, 0,358.000000")))

(event EventOpenDoor
  (Audio|Components|Audio|Play (Variables|Default|GetDoor-opening) 0.0)
  (Components|Activation|Deactivate (Variables|Default|GetParticleSystem))
  (bind _open_door_track (Timeline|Timeline_0 PlayFromStart)
    (:Update
      (Transformation|SetActorLocation (Math|Vector|Lerp(Vector) (Variables|Default|GetInitPos) (Variables|Default|GetFinalPos) _open_door_track) false false))))

(fn ConstructionScript
  (|CallParentFunction))