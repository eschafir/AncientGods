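; A floor button actor that opens a linked Door when its box is overlapped, serving as either the level's initial or final door switch.
; The initial button also starts the level countdown in the player's UI; the final one requires all stars collected, otherwise playing an error sound and Timeline-faded warning.
; Activation lowers the button, swaps its material, stops its particles and blocks retriggering, while a DoOnce reset on end overlap allows retries after failure.
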(event OnComponentEndOverlap(Box)
  (params (OverlappedComponent :type Primitive%20Component%20Object%20Reference) (OtherActor :type Actor%20Object%20Reference) (OtherComp :type Primitive%20Component%20Object%20Reference) (OtherBodyIndex :type Integer))
  (Utilities|FlowControl|DoOnce false) ; enters at Reset
)

(event OnComponentBeginOverlap(Box)
  (params (OverlappedComponent :type Primitive%20Component%20Object%20Reference) (OtherActor :type Actor%20Object%20Reference) (OtherComp :type Primitive%20Component%20Object%20Reference) (OtherBodyIndex :type Integer) (bFromSweep :type Boolean) (SweepResult :type Hit%20Result%20Structure%20%28by%20ref%29))
  (if (not (Variables|Default|GetisActivated))
    (Utilities|FlowControl|DoOnce false
      (:Completed
        (Audio|Components|Audio|Play (Variables|Default|GetButton) 0.0)
        (if (Variables|Default|GetisInitialDoor)
          (CallFunction|EventOpenInitialDoor)
          (else
            (CallFunction|EventOpenFinalDoor)))))))

(event Custom|Event%20Open%20Initial%20Door
  ;[1 1 1] Open the initial door of the level
  (CallFunction|ActivateButton)
  (Default|OpenDoor (.AsDoor (Utilities|Casting|CastToDoor (Variables|Default|Getopen%20Door))))
  (bind _asfirst_person_character (Utilities|Casting|CastToFirstPersonCharacter (Game|GetPlayerCharacter 0)))
  (Default|BeginCount (Variables|/Game/FirstPersonBP/Blueprints/FirstPersonCharacter.FirstPersonCharacter_C|GetCharacterUI _asfirst_person_character) (Variables|Default|GetLevelTime)))

(event Custom|Event%20Open%20Final%20Door
  (bind _returnvalue (Game|GetPlayerCharacter 0))
  (bind _returnvalue_2 (Game|GetPlayerCharacter 0))
  (bind _asfirst_person_character (Utilities|Casting|CastToFirstPersonCharacter _returnvalue))
  (bind _asfirst_person_character_2 (Utilities|Casting|CastToFirstPersonCharacter _returnvalue_2))
  (bind _characterui (Variables|/Game/FirstPersonBP/Blueprints/FirstPersonCharacter.FirstPersonCharacter_C|GetCharacterUI _asfirst_person_character_2))
  (bind _characterui_2 (Variables|/Game/FirstPersonBP/Blueprints/FirstPersonCharacter.FirstPersonCharacter_C|GetCharacterUI _asfirst_person_character))
  (bind _warningtext (Variables|/Game/TheStarter/UI/PlayerUI.PlayerUI_C|GetWarningText _characterui))
  (bind _warningtext_2 (Variables|/Game/TheStarter/UI/PlayerUI.PlayerUI_C|GetWarningText _characterui_2))
  ;[1 1 1] Open the final door of the level
  (bind _bool (CallFunction|PlayerHasAllPickups))
  (if _bool
    (Utilities|FlowControl|DoOnce false
      (:Completed
        (CallFunction|ActivateButton)
        (Default|OpenDoor (.AsDoor (Utilities|Casting|CastToDoor (Variables|Default|Getopen%20Door))))))
    (else
      (Audio|Components|Audio|Play (Variables|Default|GetError) 0.0)
      (Rendering|Components|TextRender|SetText _warningtext (Utilities|Text|ToText(String) "You have to find all the items."))
      (Widget|SetVisibility _warningtext "Visible")
      (bind _newtrack_0 (Timeline|Timeline_0 PlayFromStart)
        (:Update
          (Appearance|SetColorandOpacity _warningtext_2 (Utilities|Struct|MakeSlateColor (Math|Color|Lerp(LinearColor) "(R=1.000000,G=0.223228,B=0.000000,A=0.000000)" "(R=1.000000,G=0.222321,B=0.000000,A=1.000000)" _newtrack_0)) :!class /Script/UMG.TextBlock))
        (:Finished
          (Widget|SetVisibility _warningtext_2 "Hidden"))))))

(fn ConstructionScript)

(fn ActivateButton
  (Utilities|FlowControl|DoOnce false
    (:Completed
      (Transformation|AddActorLocalOffset "0, 0,-2.000000" false false)
      (Rendering|Material|SetMaterial (Variables|Default|GetStaticMesh) 0 "/Game/TheStarter/Materials/Button_activated.Button_activated")
      (Components|Activation|Deactivate (Variables|Default|GetParticleSystem))
      (Variables|Default|SetisActivated true))))

(fn PlayerHasAllPickups
  (bind _returnvalue (Game|GetPlayerCharacter 0))
  (bind _asfirst_person_character (Utilities|Casting|CastToFirstPersonCharacter _returnvalue))
  (return (== (Variables|/Game/FirstPersonBP/Blueprints/FirstPersonCharacter.FirstPersonCharacter_C|GetStarsCollected _asfirst_person_character) (Variables|/Game/FirstPersonBP/Blueprints/FirstPersonCharacter.FirstPersonCharacter_C|GetTotalStarsInLevel _asfirst_person_character))))